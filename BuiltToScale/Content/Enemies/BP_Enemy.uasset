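; BP_Enemy is an enemy character that chases the BP_Ortiz actor and drops a BP_Pickup when it dies.
; Every Tick it looks up BP_Ortiz and issues a simple AI move toward it, rotating to face its movement.
; Any damage sets Life to Damage minus Life (operands reversed from a usual subtraction), and at zero or below it spawns the pickup and destroys itself.
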(event EventBeginPlay
  (Variables|/Script/Engine.CharacterMovementComponent|SetbOrientRotationToMovement (Variables|Character|GetCharacterMovement) true))

(event Collision|EventActorBeginOverlap
  (params (OtherActor :type Actor%20Object%20Reference)))

(event EventTick
  (params (DeltaSeconds :type Float%20%28single-precision%29))
  (bind _returnvalue (Actor|GetActorOfClass "/Game/Characters/Ortiz/BP_Ortiz.BP_Ortiz_C"))
  (AI|Navigation|SimpleMovetoActor (AI|GetAIController self) _returnvalue))

(event Game|Damage|EventAnyDamage
  (params (Damage :type Float%20%28single-precision%29) (DamageType :type Damage%20Type%20Object%20Reference) (InstigatedBy :type Controller%20Object%20Reference) (DamageCauser :type Actor%20Object%20Reference))
  (bind _output_get (Variables|Default|SetLife (- Damage (Variables|Default|GetLife))))
  (if (<= _output_get 0.0)
    (Game|SpawnActorfromClass "/Game/Pickups/BP_Pickup.BP_Pickup_C" (Transformation|GetActorTransform self) "Undefined" "MultiplyWithRoot" 0 0)
    (Actor|DestroyActor)))

(fn ConstructionScript)