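; BP_Dragon is an enemy character that chases BP_Ortiz and plays an attack animation when close.
; Each tick, unless attacking, it issues AIMoveTo toward Ortiz until within a range that grows with Ortiz's scale factor.
; In range, it stops and plays the attack montage, holding IsAttacking until the montage completes.
; Life is initialized on BeginPlay but unused here, and no damage logic is present.
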(event EventTick
  (params (DeltaSeconds :type Float%20%28single-precision%29))
  (if (not (Variables|Default|GetIsAttacking))
    (bind _returnvalue (Actor|GetActorOfClass "/Game/Characters/Ortiz/BP_Ortiz.BP_Ortiz_C"))
    (if (<= (Transformation|GetDistanceTo _returnvalue) (* (Variables|/Game/Characters/Ortiz/BP_Ortiz.BP_Ortiz_C|GetCurrentScaleFactor _returnvalue) 3e+02))
      (Components|Movement|StopMovementImmediately (Variables|Character|GetCharacterMovement))
      (Variables|Default|SetIsAttacking true)
      (Animation|Montage|PlayMontage (Variables|Character|GetMesh) "/Game/Enemies/Dragon/AM_Attack.AM_Attack"
        (:OnCompleted
          (Variables|Default|SetIsAttacking false)))
      (else
        (AI|AIMoveTo self "0, 0, 0" _returnvalue 1.5e+02 false)))))

(event EventBeginPlay
  (Variables|/Script/Engine.CharacterMovementComponent|SetbOrientRotationToMovement (Variables|Character|GetCharacterMovement) true)
  (Variables|Default|SetLife 1e+01))

(fn ConstructionScript)