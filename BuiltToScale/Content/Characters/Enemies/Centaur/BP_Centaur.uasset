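; BP_Centaur is a melee enemy that chases BP_Ortiz, assembled from modular skeletal meshes that follow the main mesh's pose.
; Tick drives AIMoveTo until within an attack range that grows with the target's AppleCount, then plays an attack montage gated by IsAttacking.
; Damage also sets IsAttacking and reduces Life; at zero it disables collision, plays a death animation, spawns BP_Pickup and destroys itself.
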(event EventBeginPlay
  (|CallParentFunction)
  (Variables|/Script/Engine.CharacterMovementComponent|SetbOrientRotationToMovement (Variables|Character|GetCharacterMovement) true)
  (Variables|Default|SetLife 1e+01)
  (Components|SkinnedMesh|SetLeaderPoseComponent (Variables|Default|GetSK_Arrow_Action) (Variables|Character|GetMesh) false false)
  (Transformation|SetWorldScale3D (Variables|Default|GetCapsuleComponent) "1.500000,1.500000,1.500000"))

(event EventTick
  (params (DeltaSeconds :type Float%20%28single-precision%29))
  (if (not (Variables|Default|GetIsAttacking))
    (bind _returnvalue (Actor|GetActorOfClass "/Game/Characters/Ortiz/BP_Ortiz.BP_Ortiz_C"))
    (if (<= (Transformation|GetDistanceTo _returnvalue) (+ (* (Variables|/Game/Characters/Ortiz/BP_Ortiz.BP_Ortiz_C|GetAppleCount _returnvalue) 8) 350))
      (Components|Movement|StopMovementImmediately (Variables|Character|GetCharacterMovement))
      (Variables|Default|SetIsAttacking true)
      (Animation|Montage|PlayMontage (Variables|Character|GetMesh) "/Game/Characters/Enemies/Centaur/AM_Attack.AM_Attack"
        (:OnCompleted
          (Utilities|FlowControl|Delay 0.5)
          (Variables|Default|SetIsAttacking false)))
      (else
        (AI|AIMoveTo self "0, 0, 0" _returnvalue (Math|Conversions|ToFloat(Integer) (+ (* (Variables|/Game/Characters/Ortiz/BP_Ortiz.BP_Ortiz_C|GetAppleCount _returnvalue) 8) 0)) false)))))

(event Game|Damage|EventAnyDamage
  (params (Damage :type Float%20%28single-precision%29) (DamageType :type Damage%20Type%20Object%20Reference) (InstigatedBy :type Controller%20Object%20Reference) (DamageCauser :type Actor%20Object%20Reference))
  (bind _mesh (Variables|Character|GetMesh))
  (Variables|Default|SetIsAttacking true)
  (bind _output_get (Variables|Default|SetLife (- (Variables|Default|GetLife) Damage)))
  (if (<= _output_get 0.0)
    (Collision|SetCollisionEnabled (Variables|Default|GetAttackHitbox) "NoCollision")
    (Collision|SetCollisionEnabled (Variables|Default|GetCapsuleComponent) "NoCollision")
    (Collision|SetCollisionEnabled _mesh "NoCollision")
    (Components|Animation|PlayAnimation _mesh "/Game/QuadrapedCreatures/Centaur/Animations/ANIM_Centaur_DeathSword.ANIM_Centaur_DeathSword" false)
    (Utilities|FlowControl|Delay 2.0)
    (Game|SpawnActorfromClass "/Game/Pickups/BP_Pickup.BP_Pickup_C" (Transformation|GetActorTransform self) "Undefined" "MultiplyWithRoot" 0 0)
    (Actor|DestroyActor)))

(fn ConstructionScript)