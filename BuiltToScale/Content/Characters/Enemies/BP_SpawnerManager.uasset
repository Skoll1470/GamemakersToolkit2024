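; Manager actor that escalates enemy waves from Barghest to Centaur to Griffon to Dragon as the player's AppleCount rises.
; Tick polls BP_Ortiz's count against fixed thresholds, using one-shot flags per stage.
; Each new stage destroys the previous enemies and spawners, then places new spawners and adds an alert widget per TargetPoint.
; The final stage instead moves an existing BP_Dragon to the DragonSpawn actor.
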(event EventBeginPlay
  (bind _outactors (Actor|GetAllActorsOfClass "/Script/Engine.TargetPoint"))
  (Variables|Default|SetTargetPoints _outactors)
  (bind _returnvalue (Actor|GetActorOfClass "/Game/Characters/Ortiz/BP_Ortiz.BP_Ortiz_C"))
  (Variables|Default|SetCharacter _returnvalue)
  (Variables|Default|SetBarghestActivated false)
  (Variables|Default|SetCentaurActivated false)
  (Variables|Default|SetGriffonActivated false)
  (Variables|Default|SetDragonActivated false))

(event EventTick
  (params (DeltaSeconds :type Float%20%28single-precision%29))
  (bind _output_get (Variables|Default|SetAppleCount (Variables|/Game/Characters/Ortiz/BP_Ortiz.BP_Ortiz_C|GetAppleCount (Variables|Default|GetCharacter))))
  (if (== _output_get 0)
    (if (not (Variables|Default|GetBarghestActivated))
      (for _array_element (Variables|Default|GetTargetPoints)
        (Game|SpawnActorfromClass "/Game/Characters/Enemies/Spawners/BP_BarghestSpawner.BP_BarghestSpawner_C" (Transformation|GetActorTransform _array_element) "Undefined" "MultiplyWithRoot" 0 0)
        (bind _returnvalue (UserInterface|CreateWidget "/Game/UI/WBP_NewEnemiesSpawn.WBP_NewEnemiesSpawn_C"))
        (UserInterface|Viewport|AddtoViewport _returnvalue 0))
      (Variables|Default|SetBarghestActivated true))
    (elif (== _output_get 10)
      (if (not (Variables|Default|GetCentaurActivated))
        (bind _outactors (Actor|GetAllActorsOfClass "/Game/Characters/Enemies/Barghest/BP_Barghest.BP_Barghest_C"))
        (for _array_element_2 _outactors
          (Actor|DestroyActor _array_element_2))
        (bind _outactors_2 (Actor|GetAllActorsOfClass "/Game/Characters/Enemies/Spawners/BP_BarghestSpawner.BP_BarghestSpawner_C"))
        (for _array_element_3 _outactors_2
          (Actor|DestroyActor _array_element_3))
        (for _array_element_4 (Variables|Default|GetTargetPoints)
          (Game|SpawnActorfromClass "/Game/Characters/Enemies/Spawners/BP_CentaurSpawner.BP_CentaurSpawner_C" (Transformation|GetActorTransform _array_element_4) "Undefined" "MultiplyWithRoot" 0 0)
          (bind _returnvalue_2 (UserInterface|CreateWidget "/Game/UI/WBP_NewEnemiesSpawn.WBP_NewEnemiesSpawn_C"))
          (UserInterface|Viewport|AddtoViewport _returnvalue_2 0))
        (Variables|Default|SetCentaurActivated true))
      (elif (== _output_get 20)
        (if (not (Variables|Default|GetGriffonActivated))
          (bind _outactors_3 (Actor|GetAllActorsOfClass "/Game/Characters/Enemies/Centaur/BP_Centaur.BP_Centaur_C"))
          (for _array_element_5 _outactors_3
            (Actor|DestroyActor _array_element_5))
          (bind _outactors_4 (Actor|GetAllActorsOfClass "/Game/Characters/Enemies/Spawners/BP_CentaurSpawner.BP_CentaurSpawner_C"))
          (for _array_element_6 _outactors_4
            (Actor|DestroyActor _array_element_6))
          (for _array_element_7 (Variables|Default|GetTargetPoints)
            (Game|SpawnActorfromClass "/Game/Characters/Enemies/Spawners/BP_GriffonSpawner.BP_GriffonSpawner_C" (Transformation|GetActorTransform _array_element_7) "Undefined" "MultiplyWithRoot" 0 0)
            (bind _returnvalue_3 (UserInterface|CreateWidget "/Game/UI/WBP_NewEnemiesSpawn.WBP_NewEnemiesSpawn_C"))
            (UserInterface|Viewport|AddtoViewport _returnvalue_3 0))
          (Variables|Default|SetGriffonActivated true))
        (elif (== _output_get 30)
          (if (not (Variables|Default|GetDragonActivated))
            (bind _outactors_5 (Actor|GetAllActorsOfClass "/Game/Characters/Enemies/Griffon/BP_Griffon.BP_Griffon_C"))
            (for _array_element_8 _outactors_5
              (Actor|DestroyActor _array_element_8))
            (bind _outactors_6 (Actor|GetAllActorsOfClass "/Game/Characters/Enemies/Spawners/BP_GriffonSpawner.BP_GriffonSpawner_C"))
            (for _array_element_9 _outactors_6
              (Actor|DestroyActor _array_element_9))
            (bind _returnvalue_4 (Actor|GetActorOfClass "/Game/Characters/Enemies/DragonSpawn.DragonSpawn_C"))
            (bind _returnvalue_5 (Actor|GetActorOfClass "/Game/Characters/Enemies/Dragon/BP_Dragon.BP_Dragon_C"))
            (Transformation|SetActorTransform _returnvalue_5 (Transformation|GetActorTransform _returnvalue_4))
            (Variables|Default|SetDragonActivated true)))))))

(fn ConstructionScript)