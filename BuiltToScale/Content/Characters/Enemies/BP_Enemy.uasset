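; BP_Enemy is an enemy that chases BP_Ortiz and damages it through an attack hitbox.
; Every Tick looks up the BP_Ortiz actor and issues a SimpleMoveToActor through the enemy's AI controller.
; An AttackHitbox overlap with BP_Ortiz applies DamageValue as damage.
; The hitbox collision is disabled on BeginPlay, and nothing in this Blueprint re-enables it.
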(event OnComponentBeginOverlap(AttackHitbox)
  (params (OverlappedComponent :type Primitive%20Component%20Object%20Reference) (OtherActor :type Actor%20Object%20Reference) (OtherComp :type Primitive%20Component%20Object%20Reference) (OtherBodyIndex :type Integer) (bFromSweep :type Boolean) (SweepResult :type Hit%20Result%20Structure%20%28by%20ref%29))
  (bind _asbp_ortiz (Utilities|Casting|CastToBP_Ortiz OtherActor))
  (Game|Damage|ApplyDamage _asbp_ortiz (Variables|Default|GetDamageValue) 0 0))

(event EventBeginPlay
  (Collision|SetCollisionEnabled (Variables|Default|GetAttackHitbox) "NoCollision"))

(event Collision|EventActorBeginOverlap
  (params (OtherActor :type Actor%20Object%20Reference)))

(event EventTick
  (params (DeltaSeconds :type Float%20%28single-precision%29))
  (bind _returnvalue (Actor|GetActorOfClass "/Game/Characters/Ortiz/BP_Ortiz.BP_Ortiz_C"))
  (AI|Navigation|SimpleMovetoActor (AI|GetAIController self) _returnvalue))

(fn ConstructionScript)