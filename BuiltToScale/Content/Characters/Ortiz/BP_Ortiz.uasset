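; BP_Ortiz is the player character, a melee fighter who grows by eating apple pickups.
; Punch and smash inputs activate GAS abilities when not already attacking, and separate arm and smash hitboxes damage enemies on overlap.
; Pickups enlarge the capsule, lengthen the camera boom, count apples and restore Life below 100.
; Damage cancels the attack and plays a hit reaction, or a death montage leading to a paused game-over screen.
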(event OnComponentBeginOverlap(CapsuleComponent)
  (params (OverlappedComponent :type Primitive%20Component%20Object%20Reference) (OtherActor :type Actor%20Object%20Reference) (OtherComp :type Primitive%20Component%20Object%20Reference) (OtherBodyIndex :type Integer) (bFromSweep :type Boolean) (SweepResult :type Hit%20Result%20Structure%20%28by%20ref%29))
  (bind _asbp_pickup (Utilities|Casting|CastToBP_Pickup OtherActor))
  (Actor|DestroyActor _asbp_pickup)
  (bind _output_get (Variables|Default|SetCurrentScaleFactor (+ (Variables|Default|GetCurrentScaleFactor) 0.1)))
  (Transformation|SetWorldScale3D (Variables|Default|GetCapsuleComponent) (* _output_get "1.000000,1.000000,1.000000"))
  (Variables|/Script/Engine.SpringArmComponent|SetTargetArmLength (Variables|Default|GetCameraBoom) (* (Variables|Default|GetCurrentScaleFactor) 1.4e+03))
  (Variables|Default|SetAppleCount (+ (Variables|Default|GetAppleCount) 1))
  (Audio|PlaySoundatLocation "/Game/SFX/Eating.Eating" (Transformation|GetActorLocation) "0, 0, 0" 3.0 1.0 0.0 0 0 0 0)
  (if (< (Variables|Default|GetLife) 1e+02)
    (Variables|Default|SetLife (+ (Variables|Default|GetLife) 1e+01))))

(event OnComponentBeginOverlap(ArmHitbox)
  (params (OverlappedComponent :type Primitive%20Component%20Object%20Reference) (OtherActor :type Actor%20Object%20Reference) (OtherComp :type Primitive%20Component%20Object%20Reference) (OtherBodyIndex :type Integer) (bFromSweep :type Boolean) (SweepResult :type Hit%20Result%20Structure%20%28by%20ref%29))
  (bind _asbp_enemy (Utilities|Casting|CastToBP_Enemy OtherActor))
  (Game|Damage|ApplyDamage _asbp_enemy 1e+01 0 0))

(event OnComponentBeginOverlap(SmashHitbox)
  (params (OverlappedComponent :type Primitive%20Component%20Object%20Reference) (OtherActor :type Actor%20Object%20Reference) (OtherComp :type Primitive%20Component%20Object%20Reference) (OtherBodyIndex :type Integer) (bFromSweep :type Boolean) (SweepResult :type Hit%20Result%20Structure%20%28by%20ref%29))
  (bind _asbp_enemy (Utilities|Casting|CastToBP_Enemy OtherActor))
  (Game|Damage|ApplyDamage _asbp_enemy 2e+01 0 0))

(event Input|EnhancedActionEvents|EnhancedInputActionIA_Punch
  (params (ActionValue :type Boolean) (ElapsedSeconds :type Float%20%28double-precision%29) (TriggeredSeconds :type Float%20%28double-precision%29) (InputAction :type Input%20Action%20Object%20Reference :default "/Game/TopDown/Input/Actions/IA_Punch.IA_Punch"))
  (if (not (Variables|Default|GetIsAttacking))
    (Abilities|TryActivateAbilitybyClass (Variables|Default|GetAbilitySystem) "/Game/Abilities/GA_Punch.GA_Punch_C" true)))

(event Input|EnhancedActionEvents|EnhancedInputActionIA_Smash
  (params (ActionValue :type Boolean) (ElapsedSeconds :type Float%20%28double-precision%29) (TriggeredSeconds :type Float%20%28double-precision%29) (InputAction :type Input%20Action%20Object%20Reference :default "/Game/TopDown/Input/Actions/IA_Smash.IA_Smash"))
  (if (not (Variables|Default|GetIsAttacking))
    (Abilities|TryActivateAbilitybyClass (Variables|Default|GetAbilitySystem) "/Game/Abilities/GA_Smash.GA_Smash_C" true)))

(event EventBeginPlay
  (Variables|/Script/Engine.CharacterMovementComponent|SetbOrientRotationToMovement (Variables|Character|GetCharacterMovement self) true)
  (GameplayAbilities|GiveAbility (Variables|Default|GetAbilitySystem) "/Game/Abilities/GA_Punch.GA_Punch_C" 0 -1)
  (Collision|SetCollisionEnabled (Variables|Default|GetArmHitbox) "NoCollision")
  (Variables|Default|SetCurrentScaleFactor 1.0)
  (bind _returnvalue (UserInterface|CreateWidget "/Game/UI/WBP_HealthBar.WBP_HealthBar_C" (Game|GetPlayerController 0)))
  (UserInterface|Viewport|AddtoViewport _returnvalue 0)
  (Collision|SetCollisionEnabled (Variables|Default|GetSmashHitbox) "NoCollision")
  (GameplayAbilities|GiveAbility (Variables|Default|GetAbilitySystem) "/Game/Abilities/GA_Smash.GA_Smash_C" 0 -1)
  (Variables|Default|SetAppleCount 0))

(event Game|Damage|EventAnyDamage
  (params (Damage :type Float%20%28single-precision%29) (DamageType :type Damage%20Type%20Object%20Reference) (InstigatedBy :type Controller%20Object%20Reference) (DamageCauser :type Actor%20Object%20Reference))
  (Variables|Default|SetIsAttacking false)
  (bind _output_get (Variables|Default|SetLife (- (Variables|Default|GetLife) Damage)))
  (Components|Movement|StopMovementImmediately (Variables|Character|GetCharacterMovement))
  (Collision|SetCollisionEnabled (Variables|Default|GetArmHitbox) "NoCollision")
  (if (> _output_get 0.0)
    (Animation|Montage|PlayMontage (Variables|Character|GetMesh) "/Game/Characters/Ortiz/Animation/AM_HitReact.AM_HitReact"
      (:OnCompleted
        (Variables|/Script/Engine.CharacterMovementComponent|SetMaxWalkSpeed (Variables|Character|GetCharacterMovement) 6e+02)))
    (else
      (Collision|SetCollisionEnabled (Variables|Default|GetCapsuleComponent) "PhysicsOnly")
      (Animation|Montage|PlayMontage (Variables|Character|GetMesh) "/Game/Characters/Ortiz/Animation/AM_Death.AM_Death"
        (:OnBlendOut
          (Game|SetGamePaused true)
          (bind _returnvalue (UserInterface|CreateWidget "/Game/UI/WBP_GameOver.WBP_GameOver_C"))
          (UserInterface|Viewport|AddtoViewport _returnvalue 0))))))

(fn ConstructionScript)